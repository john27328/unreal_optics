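; Optics demo actor that traces rays off mirror triangles and draws their paths at BeginPlay.
; It builds a hard-coded ray and three BP_triangle surfaces sharing a Mirror shader, then each Ray's PathTrecking computes its bounce segments.
; Each segment spawns a BP_ray_drow actor, aimed along the ray and scaled to its length, or MaxLen without one.
; GetNormal and Intersection are zero-returning stubs, and TestRts is an unconnected single-intersection test.
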(event `self.ReceiveBeginPlay`
  (bind _newparam (`self.gen rays`))
  (bind _edges (`self.crerate optics`))
  (bind _paths (`self.raytraseDrow` _newparam _edges))
  (`self.DrowRaysPath` _paths))

(fn `crerate optics`
  (returns (edges :type "Array of /Game/Blueprints/edge/edge Object Reference"))
  (bind _returnvalue (`SceneComponent.K2_GetComponentToWorld` (`self.DefaultSceneRoot`)))
  (bind _returnvalue_2 (`|GenericCreateObject` "/Game/Blueprints/shader/Mirror.Mirror_C" self))
  (bind _returnvalue_3 (`|SpawnActorFromClass` "/Game/Blueprints/edge/BP_triangle.BP_triangle_C" _returnvalue "Undefined" "OverrideRootScale" null (-100.0 -100.0) (-100.0 100.0) (100.0 100.0) (-100.0 0.0 0.0) (0.0 0.0 -1.0) (0.0 1.0 0.0) _returnvalue_2 null))
  (bind _returnvalue_4 (`|SpawnActorFromClass` "/Game/Blueprints/edge/BP_triangle.BP_triangle_C" _returnvalue "Undefined" "OverrideRootScale" null (-100.0 -100.0) (-100.0 100.0) (100.0 100.0) (100.0 0.0 50.0) (0.0 0.0 1.0) (0.0 1.0 0.0) _returnvalue_2 null))
  (bind _returnvalue_5 (`|SpawnActorFromClass` "/Game/Blueprints/edge/BP_triangle.BP_triangle_C" _returnvalue "Undefined" "OverrideRootScale" null (-100.0 -100.0) (-100.0 100.0) (100.0 100.0) (0.0 0.0 100.0) (1.0 0.0 0.0) (0.0 1.0 0.0) _returnvalue_2 null))
  (return (`|MakeArray` _returnvalue_3 _returnvalue_4 _returnvalue_5 :!type "/Game/Blueprints/edge/edge Object Reference")))

(fn `drawRay`
  (params (ray :type "/Game/Blueprints/ray/ray Object Reference"))
  (returns (draw :type "/Game/Blueprints/ray/BP_ray_drow Object Reference"))
  (locals (len :type "Float (double-precision)" :default 100.0))
  (bind _raydiameter (`self.rayDiameter`))
  (bind _len (`/Game/Blueprints/ray/ray.len` ray))
  (if (< 0.0 _len)
    (set `local.len` (/ _len 100.0))
    (else
      (set `local.len` (`self.maxLen`))))
  (bind _returnvalue (`|SpawnActorFromClass` "/Game/Blueprints/ray/BP_ray_drow.BP_ray_drow_C" (`KismetMathLibrary.MakeTransform` (`/Game/Blueprints/ray/ray.point` ray) (`KismetMathLibrary.FindLookAtRotation` (`KismetMathLibrary.MakeVector` 0.0) (`/Game/Blueprints/ray/ray.vector` ray)) (`KismetMathLibrary.MakeVector` _raydiameter _raydiameter (`local.len`))) "Undefined" "OverrideRootScale" null null))
  (`self.K2_AddActorWorldOffset` _returnvalue (`SceneComponent.K2_GetComponentLocation` (`self.DefaultSceneRoot`)) false false)
  (return _returnvalue))

(fn `DrowRaysPath`
  (params (path :type "Array of /Game/Blueprints/ray/ray Object Reference"))
  (returns (NewParam :type "Array of /Game/Blueprints/ray/BP_ray_drow Object Reference"))
  (bind _drowarray (`self.drowArray`))
  (`KismetArrayLibrary.Array_Clear` (`self.drowArray`))
  (for _array_element path
    (bind _draw (`self.drawRay` _array_element))
    (`KismetArrayLibrary.Array_Add` _drowarray _draw))
  (return _drowarray))

(fn `gen rays`
  (returns (NewParam :type "Array of /Game/Blueprints/ray/ray Object Reference"))
  (bind _returnvalue (`|GenericCreateObject` "/Game/Blueprints/ray/ray.ray_C" self 1.0 (0.0 0.0 -20.0) (1.0 0.0 0.1)))
  (`|GenericCreateObject` "/Game/Blueprints/ray/ray.ray_C" self 1.0 (0.0 0.0 -20.0) (1.0 0.0 0.01))
  (`|GenericCreateObject` "/Game/Blueprints/ray/ray.ray_C" self 1.0 (0.0 0.0 -20.0) (1.0 -0.01 0.0))
  (return (`|MakeArray` _returnvalue)))

(fn `getNormal`
  (returns (normal :type "Vector Structure"))
  (return (0.0 0.0 0.0)))

(fn `intersection`
  (params (ray :type "/Game/Blueprints/ray/ray Object Reference"))
  (returns (len :type "Float (double-precision)") (normal :type "Vector Structure") (point :type "Vector Structure"))
  (return 0.0 (0.0 0.0 0.0) (0.0 0.0 0.0)))

(fn `raytraseDrow`
  (params (rays :type "Array of /Game/Blueprints/ray/ray Object Reference") (edges :type "Array of /Game/Blueprints/edge/edge Object Reference") (segments :type Integer :default 10))
  (returns (paths :type "Array of /Game/Blueprints/ray/ray Object Reference"))
  (locals (path :type "Array of /Game/Blueprints/ray/ray Object Reference"))
  (`KismetArrayLibrary.Array_Clear` (`local.path`))
  (for _array_element rays
    (bind _reypath (`/Game/Blueprints/ray/ray.pathTrecking` _array_element edges segments))
    (`KismetArrayLibrary.Array_Append` (`local.path`) _reypath))
  (return (`local.path`)))

(fn `testRts`
  (bind _returnvalue (`|GenericCreateObject` "/Game/Blueprints/ray/ray.ray_C" self 5.0 (-115.0 0.0 50.0) (1.0 0.0 0.0)))
  (bind _returnvalue_2 (`|GenericCreateObject` "/Game/Blueprints/shader/Mirror.Mirror_C" self))
  (bind _returnvalue_3 (`|SpawnActorFromClass` "/Game/Blueprints/edge/BP_triangle.BP_triangle_C" (`SceneComponent.K2_GetComponentToWorld` (`self.DefaultSceneRoot`)) "Undefined" "OverrideRootScale" null (-100.0 -100.0) (-100.0 100.0) (100.0 100.0) (15.0 0.0 0.0) (0.0 0.0 -1.0) (0.0 1.0 0.0) _returnvalue_2 null))
  (bind (_len _normal _point) (message `/Game/Blueprints/edge/edgeInterface.intersection` _returnvalue_3 _returnvalue))
  (`KismetSystemLibrary.PrintString` (`KismetStringLibrary.Conv_VectorToString` _point) true false (struct :`R` 1.0 :`B` 0.045081 :`A` 1.0))
  (`KismetSystemLibrary.PrintString` (`KismetStringLibrary.Conv_DoubleToString` _len) true false (struct :`R` 1.0 :`B` 0.045081 :`A` 1.0))
  (set `/Game/Blueprints/ray/ray.len` _len _returnvalue)
  (`self.drawRay` _returnvalue))

(fn `UserConstructionScript`)