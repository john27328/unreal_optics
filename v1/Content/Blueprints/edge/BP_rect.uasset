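; BP_rect is an actor meant to form a glass box sized by Width, Height and Thickness.
; Construction script and BeginPlay both call Create, but its body is empty.
; Disconnected nodes would spawn six Edge_triangle actors as faces, give each four corner points, then offset them by the actor's transform.
; Intersection and GetNormal are stubs returning zeros, so the actor currently builds and computes nothing.
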(event `self.ReceiveBeginPlay`
  (`self.create`))

(fn `create`)

(fn `getNormal`
  (returns (normal :type "Vector Structure"))
  (return (0.0 0.0 0.0)))

(fn `intersection`
  (params (ray :type "/Game/Blueprints/ray/ray Object Reference"))
  (returns (len :type "Float (double-precision)") (normal :type "Vector Structure") (point :type "Vector Structure"))
  (return 0.0 (0.0 0.0 0.0) (0.0 0.0 0.0)))

(fn `UserConstructionScript`
  (`self.create`))