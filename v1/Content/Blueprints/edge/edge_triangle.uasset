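; Triangle edge actor that renders a flat triangle and answers analytic ray-intersection queries, apparently for a custom ray tracer.
; On BeginPlay it builds a procedural mesh from three local 2D points with scaled UVs, then places it using Center and the VectorU/VectorV axes.
; It caches world-space corners and the plane normal.
; Intersection uses a ray-plane hit and cross-product barycentric test, returning distance, normal, point and Shader, or -1 on a miss.
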(event `self.ReceiveBeginPlay`
  (`parent.ReceiveBeginPlay`)
  (`self.create`))

(fn `create`
  (bind _proceduralmesh (`self.ProceduralMesh`))
  (bind _vectoru (`self.vectorU`))
  (bind _vectorv (`self.vectorV`))
  (bind _center (`self.center`))
  (bind _returnvalue (`KismetMathLibrary.MakeRotFromXY` _vectoru _vectorv))
  (bind (_vertices _triangless _uv _normals) (`self.createMash`))
  (`ProceduralMeshComponent.CreateMeshSection_LinearColor` :`self` (`self.ProceduralMesh`) :`Vertices` _vertices :`Triangles` _triangless :`Normals` _normals :`UV0` _uv)
  ;[1 1 1] поварачиваю плоскость
  (`SceneComponent.K2_AddLocalOffset` _proceduralmesh _center false false)
  (`SceneComponent.K2_AddLocalRotation` _proceduralmesh _returnvalue false false)
  (`PrimitiveComponent.SetMaterial` _proceduralmesh 0 (`self.material`))
  ;[1 1 1] задаю нормаль
  (set `self.normal` (`KismetMathLibrary.Normal` (`KismetMathLibrary.Cross_VectorVector` _vectoru _vectorv)))
  ;[1 1 1] поворот координат
  (set `self.p1Global` (+ (`KismetMathLibrary.GreaterGreater_VectorRotator` (`KismetMathLibrary.Conv_Vector2DToVector` (`self.p1_local`)) _returnvalue) _center))
  (set `self.p2Global` (+ (`KismetMathLibrary.GreaterGreater_VectorRotator` (`KismetMathLibrary.Conv_Vector2DToVector` (`self.p2_local`)) _returnvalue) _center))
  (set `self.p3Global` (+ (`KismetMathLibrary.GreaterGreater_VectorRotator` (`KismetMathLibrary.Conv_Vector2DToVector` (`self.p3_local`)) _returnvalue) _center)))

(fn `createMash`
  (returns (vertices :type "Array of Vector Structure (by ref)") (triangless :type "Array of Integer (by ref)") (UV :type "Array of Vector2D Structure (by ref)") (normals :type "Array of Vector Structure"))
  (bind _scale (`self.scale`))
  (bind _scale_2 (`self.scale`))
  (bind _scale_3 (`self.scale`))
  (bind (_p1_local_x _p1_local_y) (`KismetMathLibrary.BreakVector2D` (`self.p1_local`)))
  (bind (_p2_local_x _p2_local_y) (`KismetMathLibrary.BreakVector2D` (`self.p2_local`)))
  (bind (_p3_local_x _p3_local_y) (`KismetMathLibrary.BreakVector2D` (`self.p3_local`)))
  (bind _array (`|MakeArray` (`KismetMathLibrary.MakeVector` _p1_local_x _p1_local_y) (`KismetMathLibrary.MakeVector` _p2_local_x _p2_local_y) (`KismetMathLibrary.MakeVector` _p3_local_x _p3_local_y) :!type "Vector Structure"))
  (bind _output (`|GetArrayItem` _array))
  (bind _returnvalue (`KismetMathLibrary.Cross_VectorVector` (- (`|GetArrayItem` _array 2) _output) (- (`|GetArrayItem` _array 1) _output)))
  (return _array (`|MakeArray` 0 1 2) (`|MakeArray` (`KismetMathLibrary.MakeVector2D` (/ _p1_local_x _scale) (/ _p1_local_y _scale)) (`KismetMathLibrary.MakeVector2D` (/ _p2_local_x _scale_2) (/ _p2_local_y _scale_2)) (`KismetMathLibrary.MakeVector2D` (/ _p3_local_x _scale_3) (/ _p3_local_y _scale_3)) :!type "Vector2D Structure") (`|MakeArray` _returnvalue _returnvalue _returnvalue)))

(fn `getNormal`
  (params (point :type "Vector Structure"))
  (returns (normal :type "Vector Structure"))
  (return (`self.normal`)))

(fn `intersection`
  (params (ray :type "/Game/Blueprints/ray/ray Object Reference"))
  (returns (len :type "Float (double-precision)") (normal :type "Vector Structure") (point :type "Vector Structure") (shader :type "/Game/Blueprints/shader/shader Object Reference"))
  (locals (NewLocalVar_0 :type "Vector Structure" :default (0.0 0.0 0.0)))
  (bind _point (`/Game/Blueprints/ray/ray.point` ray))
  (bind _vector (`/Game/Blueprints/ray/ray.vector` ray))
  (bind _p1global (`self.p1Global`))
  (bind _returnvalue (- (`self.p2Global`) _p1global))
  (bind _returnvalue_2 (- (`self.p3Global`) _p1global))
  (bind _returnvalue_3 (`KismetMathLibrary.Cross_VectorVector` _returnvalue _returnvalue_2))
  (bind _returnvalue_4 (`KismetMathLibrary.Dot_VectorVector` _returnvalue_3 _returnvalue_3))
  ;[1 1 1] нахожу d = - n * r1
  (bind _normal (`self.getNormal` (0.0 0.0 0.0)))
  (bind _returnvalue_5 (`KismetMathLibrary.Dot_VectorVector` _vector _normal))
  ;[1 1 1] луч параллелен плоскости
  (if (!= _returnvalue_5 0.0)
    (bind _returnvalue_6 (/ (* -1 (+ (* -1 (`KismetMathLibrary.Dot_VectorVector` (`self.p1Global`) _normal)) (`KismetMathLibrary.Dot_VectorVector` _point _normal))) _returnvalue_5))
    ;[1 1 1] не в ту сторону
    (if (> _returnvalue_6 0.0)
      (bind _returnvalue_7 (+ _point (* _vector _returnvalue_6)))
      (bind _returnvalue_8 (- _returnvalue_7 _p1global))
      (bind _returnvalue_9 (`KismetMathLibrary.Dot_VectorVector` (`KismetMathLibrary.Cross_VectorVector` _returnvalue _returnvalue_8) _returnvalue_3))
      (bind _returnvalue_10 (`KismetMathLibrary.Dot_VectorVector` (`KismetMathLibrary.Cross_VectorVector` _returnvalue_8 _returnvalue_2) _returnvalue_3))
      ;[1 1 1] попадание в треугольник
      (if (and (`KismetMathLibrary.InRange_FloatFloat` _returnvalue_9 0.0 _returnvalue_4) (`KismetMathLibrary.InRange_FloatFloat` _returnvalue_10 0.0 _returnvalue_4) (`KismetMathLibrary.InRange_FloatFloat` (+ _returnvalue_9 _returnvalue_10) 0.0 _returnvalue_4))
        (return (`KismetMathLibrary.Vector_Distance` _returnvalue_7 _point) _normal _returnvalue_7 (`self.shader`))
        (else
          _))))
  (return -1.0 (0.0 0.0 0.0) (0.0 0.0 0.0) null))

(fn `UserConstructionScript`)