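; Spherical sector surface actor that draws itself and answers ray intersection queries, returning distance, normal, point and shader.
; On BeginPlay, Create builds a latitude-longitude procedural mesh between two polar angles, then offsets it to Center and orients it by VectorU and VectorV.
; Intersection solves the ray-sphere quadratic analytically and keeps the nearest forward hit beyond LMin that PointOnSector places within the band along RadiusVector, otherwise returning length -1.
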(event `self.ReceiveBeginPlay`
  (`parent.ReceiveBeginPlay`)
  (`self.create`))

(fn `alpha_i`
  (params (i :type "Integer (by ref)"))
  (returns (angle :type "Float (double-precision)"))
  (bind _anglestart (`self.angleStart`))
  (return (+ (+ _anglestart 1.0) (* (/ (- (`self.angleEnd`) _anglestart) (`KismetMathLibrary.Conv_IntToDouble` (`self.alphaSections`))) (`KismetMathLibrary.Conv_IntToDouble` i)))))

(fn `create`
  (bind _proceduralmesh (`self.ProceduralMesh`))
  (bind _alphasections (`self.alphaSections`))
  (bind _radius (`self.radius`))
  (bind _thetasections (`self.thetaSections`))
  (bind _vertics (`self.vertics`))
  (bind _trifngles (`self.trifngles`))
  (`KismetArrayLibrary.Array_Clear` (`self.vertics`))
  (`KismetArrayLibrary.Array_Clear` (`self.trifngles`))
  (for _index (range (+ _alphasections 1))
    (for _index_2 (range _thetasections)
      (`KismetArrayLibrary.Array_Append` _vertics (`|MakeArray` (`self.p_i_j` _index _index_2)))))
  (for _index_3 (range _alphasections)
    (for _index_4 (range (+ _thetasections 1))
      (bind _n (`self.i_j_to_n` _index_3 _index_4))
      (bind _returnvalue (+ _index_3 1))
      (bind _returnvalue_2 (+ _index_4 1))
      (bind _n_2 (`self.i_j_to_n` _returnvalue _returnvalue_2))
      (`KismetArrayLibrary.Array_Append` _trifngles (`|MakeArray` _n (`self.i_j_to_n` _returnvalue _index_4) _n_2 _n _n_2 (`self.i_j_to_n` _index_3 _returnvalue_2)))))
  (`ProceduralMeshComponent.CreateMeshSection_LinearColor` :`self` (`self.ProceduralMesh`) :`Vertices` _vertics :`Triangles` _trifngles)
  ;[1 1 1] поварачиваю плоскость
  (`SceneComponent.K2_AddLocalOffset` _proceduralmesh (`self.center`) false false)
  (`SceneComponent.K2_AddLocalRotation` _proceduralmesh (`KismetMathLibrary.MakeRotFromXY` (`self.vectorU`) (`self.vectorV`)) false false)
  (`PrimitiveComponent.SetMaterial` _proceduralmesh 0 (`self.material`))
  ;[1 1 1] вектор, указывающий вперед длинной в радиус
  (set `self.radiusVector` (`KismetMathLibrary.Normal` (`KismetMathLibrary.Cross_VectorVector` (`self.vectorU`) (`self.vectorV`))))
  (set `self.startR` (* _radius (`KismetMathLibrary.DegCos` (`self.angleStart`))))
  (set `self.endR` (* _radius (`KismetMathLibrary.DegCos` (`self.angleEnd`)))))

(fn `getNormal`
  (params (point :type "Vector Structure"))
  (returns (normal :type "Vector Structure"))
  (return (`KismetMathLibrary.Normal` (- point (`self.center`)))))

(fn `i_j_to_n`
  (params (i :type "Integer (by ref)") (j :type "Integer (by ref)"))
  (returns (n :type Integer))
  (locals (iTmp :type Integer) (jTmp :type Integer))
  (bind _thetasections (`self.thetaSections`))
  (set `local.iTmp` i)
  (set `local.jTmp` j)
  (if (not (< (`local.jTmp`) _thetasections))
    (set `local.jTmp` 0))
  (return (+ (`local.jTmp`) (* _thetasections (`local.iTmp`)))))

(fn `intersection`
  (params (ray :type "/Game/Blueprints/ray/ray Object Reference"))
  (returns (len :type "Float (double-precision)") (normal :type "Vector Structure") (point :type "Vector Structure") (shader :type "/Game/Blueprints/shader/shader Object Reference"))
  (bind _lmin (`self.lMin`))
  (bind _point (`/Game/Blueprints/ray/ray.point` ray))
  (bind _vector (`/Game/Blueprints/ray/ray.vector` ray))
  (bind _radius (`self.radius`))
  (bind _shader (`self.shader`))
  (bind _returnvalue (- _point (`self.center`)))
  (bind _returnvalue_2 (* (`KismetMathLibrary.Dot_VectorVector` _returnvalue _vector) 2.0))
  (bind _returnvalue_3 (/ (* -1 _returnvalue_2) 2.0))
  (bind _returnvalue_4 (- (/ (* _returnvalue_2 _returnvalue_2) 4.0) (- (`KismetMathLibrary.Dot_VectorVector` _returnvalue _returnvalue) (* _radius _radius))))
  (bind _returnvalue_5 (`KismetMathLibrary.Sqrt` _returnvalue_4))
  (bind _returnvalue_6 (- _returnvalue_3 _returnvalue_5))
  (bind _returnvalue_7 (+ _returnvalue_3 _returnvalue_5 0.0))
  (bind _returnvalue_8 (+ _point (* _vector _returnvalue_7)))
  (bind _returnvalue_9 (+ _point (* _vector _returnvalue_6)))
  (bind _returnvalue_10 (`KismetMathLibrary.VSize` (- _returnvalue_8 _point)))
  (bind _returnvalue_11 (`KismetMathLibrary.VSize` (- _returnvalue_9 _point)))
  (bind _returnvalue_12 (and (`self.pointOnSector` _returnvalue_9) (> _returnvalue_6 0.0) (> _returnvalue_11 _lmin)))
  (bind _returnvalue_13 (and (`self.pointOnSector` _returnvalue_8) (> _returnvalue_7 0.0) (> _returnvalue_10 _lmin)))
  (if (> _returnvalue_4 0.0)
    ;[1 1 1] ищу первую точку
    (if (and _returnvalue_12 _returnvalue_13)
      (if (< _returnvalue_11 _returnvalue_10)
        (bind _normal (`/Game/Blueprints/edge/edgeInterface.getNormal` _returnvalue_9 :!label _label))
        (return _returnvalue_11 _normal _returnvalue_9 _shader)
        (else
          (bind _normal_2 (`/Game/Blueprints/edge/edgeInterface.getNormal` _returnvalue_8 :!label _label_2))
          (return _returnvalue_10 _normal_2 _returnvalue_8 _shader)))
      (elif (and _returnvalue_12 (not _returnvalue_13))
        (goto _label)
        (elif (and (not _returnvalue_12) _returnvalue_13)
          (goto _label_2)
          (else
            _)))))
  (return -1.0 (0.0 0.0 0.0) (0.0 0.0 0.0) _shader))

(fn `p_i_j`
  (params (i :type "Integer (by ref)") (j :type "Integer (by ref)"))
  (returns (NewParam :type "Vector Structure"))
  (bind _angle (`self.alpha_i` i))
  (bind _angle_2 (`self.theta_i` j))
  (bind _radius (`self.radius`))
  (return (`KismetMathLibrary.MakeVector` (* _radius (`KismetMathLibrary.DegSin` _angle) (`KismetMathLibrary.DegSin` _angle_2)) (* _radius (`KismetMathLibrary.DegSin` _angle) (`KismetMathLibrary.DegCos` _angle_2)) (* _radius (`KismetMathLibrary.DegCos` _angle)))))

(fn `pointOnSector`
  (params (point :type "Vector Structure"))
  (returns (true :type Boolean))
  (bind _returnvalue (`KismetMathLibrary.Dot_VectorVector` (- point (`self.center`)) (`self.radiusVector`)))
  (return (and (<= _returnvalue (`self.startR`)) (>= _returnvalue (`self.endR`)))))

(fn `theta_i`
  (params (i :type "Integer (by ref)"))
  (returns (angle :type "Float (double-precision)"))
  (return (* i (/ 360.0 (`KismetMathLibrary.Conv_IntToDouble` (`self.thetaSections`))))))

(fn `UserConstructionScript`
  (`parent.UserConstructionScript`))