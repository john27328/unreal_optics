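; BP_quadrangle is a planar glass surface that, despite its name, builds a single procedural triangle from three local 2D points.
; Construction orients the mesh by XVector and YVector, offsets it by Vector, and caches the plane normal and first world point.
; Intersection tests a ray against that infinite plane, returning Len -1 for parallel or non-forward hits.
; The hit case is unfinished: its point calculation is unconnected.
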(event `self.ReceiveBeginPlay`)

(fn `create`
  (bind _proceduralmesh (`self.ProceduralMesh`))
  (bind _vector (`self.vector`))
  (bind _xvector (`self.xVector`))
  (bind _yvector (`self.yVector`))
  (bind _scale (`self.scale`))
  (bind _scale_2 (`self.scale`))
  (bind _scale_3 (`self.scale`))
  (bind (_p1_local_x _p1_local_y) (`KismetMathLibrary.BreakVector2D` (`self.p1_local`)))
  (bind (_p2_local_x _p2_local_y) (`KismetMathLibrary.BreakVector2D` (`self.p2_local`)))
  (bind (_p3_local_x _p3_local_y) (`KismetMathLibrary.BreakVector2D` (`self.p3_local`)))
  (bind _returnvalue (`KismetMathLibrary.MakeRotFromXY` _xvector _yvector))
  (`ProceduralMeshComponent.CreateMeshSection_LinearColor` :`self` _proceduralmesh :`Vertices` (`|MakeArray` (`KismetMathLibrary.MakeVector` _p1_local_x _p1_local_y) (`KismetMathLibrary.MakeVector` _p2_local_x _p2_local_y) (`KismetMathLibrary.MakeVector` _p3_local_x _p3_local_y) :!type "Vector Structure") :`Triangles` (`|MakeArray` 0 1 2) :`UV0` (`|MakeArray` (`KismetMathLibrary.MakeVector2D` (/ _p1_local_x _scale) (/ _p1_local_y _scale)) (`KismetMathLibrary.MakeVector2D` (/ _p2_local_x _scale_2) (/ _p2_local_y _scale_2)) (`KismetMathLibrary.MakeVector2D` (/ _p3_local_x _scale_3) (/ _p3_local_y _scale_3)) :!type "Vector2D Structure"))
  ;[1 1 1] поварачиваю плоскость
  (`SceneComponent.K2_AddWorldRotation` _proceduralmesh _returnvalue false false)
  (`SceneComponent.K2_AddWorldOffset` _proceduralmesh _vector false false)
  (`PrimitiveComponent.SetMaterial` _proceduralmesh 0 "/Game/StarterContent/Materials/M_Glass.M_Glass")
  ;[1 1 1] задаю нормаль
  (set `self.normal` (`KismetMathLibrary.Normal` (`KismetMathLibrary.Cross_VectorVector` _xvector _yvector)))
  ;[1 1 1] нахожу 1 точку на плоскости
  (set `self.p1Global` (+ (`KismetMathLibrary.GreaterGreater_VectorRotator` (`KismetMathLibrary.Conv_Vector2DToVector` (`self.p1_local`)) _returnvalue) _vector)))

(fn `getNormal`
  (returns (normal :type "Vector Structure"))
  (return (`self.normal`)))

(fn `intersection`
  (params (ray :type "/Game/Blueprints/ray/ray Object Reference"))
  (returns (len :type "Float (double-precision)") (normal :type "Vector Structure") (point :type "Vector Structure"))
  ;[1 1 1] нахожу d = - n * r1
  (bind _normal (`self.getNormal`))
  (bind _returnvalue (`KismetMathLibrary.Dot_VectorVector` (`/Game/Blueprints/ray/ray.vector` ray) _normal))
  ;[1 1 1] луч параллелен плоскости
  (if (!= _returnvalue 0.0)
    ;[1 1 1] не в ту сторону
    (if (not (> (/ (* -1 (+ (* -1 (`KismetMathLibrary.Dot_VectorVector` (`self.p1Global`) _normal)) (`KismetMathLibrary.Dot_VectorVector` (`/Game/Blueprints/ray/ray.point` ray) _normal))) _returnvalue) 0.0))
      (return -1.0 (0.0 0.0 0.0) (0.0 0.0 0.0)))
    (else
      (return -1.0 (0.0 0.0 0.0) (0.0 0.0 0.0)))))

(fn `UserConstructionScript`
  (`self.create`))