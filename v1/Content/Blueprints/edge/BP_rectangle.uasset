(fn `create`
  (bind _returnvalue (/ (`self.diabeterU`) 2.0))
  (bind _returnvalue_2 (/ (`self.diameterV`) 2.0))
  (bind _returnvalue_3 (`SceneComponent.K2_GetComponentToWorld` (`self.DefaultSceneRoot`)))
  (bind _returnvalue_4 (/ (`self.diabeterU`) 2.0))
  (bind _returnvalue_5 (/ (`self.diameterV`) 2.0))
  (bind _returnvalue_6 (* _returnvalue_4 -1.0))
  (bind _returnvalue_7 (* _returnvalue_5 -1.0))
  (bind _returnvalue_8 (`|SpawnActorFromClass` "/Game/Blueprints/edge/BP_triangle.BP_triangle_C" _returnvalue_3 "Undefined" "OverrideRootScale" null (`KismetMathLibrary.MakeVector2D` _returnvalue_6 _returnvalue_5) (`KismetMathLibrary.MakeVector2D` _returnvalue_6 _returnvalue_7) (`KismetMathLibrary.MakeVector2D` _returnvalue_4 _returnvalue_7) (`self.center`) (`self.U`) (`self.V`) (`self.ShaderIn`) null))
  (bind _returnvalue_9 (`|SpawnActorFromClass` "/Game/Blueprints/edge/BP_triangle.BP_triangle_C" _returnvalue_3 "Undefined" "OverrideRootScale" null (`KismetMathLibrary.MakeVector2D` (* _returnvalue -1.0) _returnvalue_2) (`KismetMathLibrary.MakeVector2D` _returnvalue _returnvalue_2) (`KismetMathLibrary.MakeVector2D` _returnvalue (* _returnvalue_2 -1.0)) (`self.center`) (`self.U`) (`self.V`) null null))
  (set `self.edges` (`|MakeArray` _returnvalue_8 _returnvalue_9)))

(fn `UserConstructionScript`
  (`parent.UserConstructionScript`))