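; Edge rectangle actor that forms a rectangular surface for ray intersection tests from two triangles.
; On BeginPlay it spawns two Edge_triangle actors split along a diagonal, with corners from half of DiameterU and DiameterV, passing on its center, U/V vectors, shader and material.
; Intersection hands both triangles to the ray's ReyTrassing call and returns length, normal and point, along with the rectangle's own Shader.
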(event `self.ReceiveBeginPlay`
  (`parent.ReceiveBeginPlay`)
  (`self.create`))

(fn `create`
  (locals (NewLocalVar_0 :type "Actor Object Reference"))
  (bind _shader (`self.shader`))
  (bind _center (`self.center`))
  (bind _material (`self.material`))
  (bind _center_2 (`self.center`))
  (bind _returnvalue (/ (`self.diameterU`) 2.0))
  (bind _returnvalue_2 (/ (`self.diameterV`) 2.0))
  (bind _returnvalue_3 (`SceneComponent.K2_GetComponentToWorld` (`self.DefaultSceneRoot`)))
  (bind _returnvalue_4 (/ (`self.diameterU`) 2.0))
  (bind _returnvalue_5 (/ (`self.diameterV`) 2.0))
  (bind _returnvalue_6 (* _returnvalue_4 -1.0))
  (bind _returnvalue_7 (* _returnvalue_5 -1.0))
  (bind _returnvalue_8 (`|SpawnActorFromClass` "/Game/Blueprints/edge/edge_triangle.edge_triangle_C" _returnvalue_3 "Undefined" "OverrideRootScale" null (`KismetMathLibrary.MakeVector2D` _returnvalue_6 _returnvalue_5) (`KismetMathLibrary.MakeVector2D` _returnvalue_6 _returnvalue_7) (`KismetMathLibrary.MakeVector2D` _returnvalue_4 _returnvalue_7) _center_2 _shader _material _center_2 (`self.vectorU`) (`self.vectorV`) null))
  (bind _returnvalue_9 (`|SpawnActorFromClass` "/Game/Blueprints/edge/edge_triangle.edge_triangle_C" _returnvalue_3 "Undefined" "OverrideRootScale" null (`KismetMathLibrary.MakeVector2D` (* _returnvalue -1.0) _returnvalue_2) (`KismetMathLibrary.MakeVector2D` _returnvalue _returnvalue_2) (`KismetMathLibrary.MakeVector2D` _returnvalue (* _returnvalue_2 -1.0)) _center _shader _material _center (`self.vectorU`) (`self.vectorV`) null))
  (set `self.poligons` (`|MakeArray` _returnvalue_8 _returnvalue_9 :!type "/Game/Blueprints/edge/edge Object Reference")))

(fn `intersection`
  (params (ray :type "/Game/Blueprints/ray/ray Object Reference"))
  (returns (len :type "Float (double-precision)") (normal :type "Vector Structure") (point :type "Vector Structure") (shader :type "/Game/Blueprints/shader/shader Object Reference"))
  (bind (_len _point _vector _normal) (`/Game/Blueprints/ray/ray.reyTrassing` ray (`self.poligons`)))
  (return _len _normal _point (`self.shader`)))

(fn `UserConstructionScript`
  (locals (NewLocalVar_1 :type "ChildActorComponent Object Reference")))