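; Ray object with a ray-tracing step that intersects the ray against a list of edges and spawns the outgoing ray.
; A linear search keeps the nearest positive-length hit and stores its distance in Len.
; Edge 0, regardless of which edge is hit, supplies the shader result that sets the new Ray's point and vector.
; With no hit, Len becomes -1 and the ray returns itself.
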(fn `reyTrassing`
  (params (edges :type "Array of ARTrackedGeometry Object Reference"))
  (returns (newRay :type "/Game/Blueprints/ray/ray Object Reference"))
  (locals (`len min` :type "Float (double-precision)" :default 0.0) (`normal min` :type "Vector Structure" :default (0.0 0.0 0.0)) (`point min` :type "Vector Structure" :default (0.0 0.0 0.0)) (`edge min` :type Integer))
  (bind _returnvalue (`KismetArrayLibrary.Array_Length` edges))
  (set `local.len min` 9.999999843067494e+17)
  (set `local.edge min` _returnvalue)
  ;[1 1 1] поиск ближайшего пересечения
  (for (_array_element _array_index) edges
    (bind (_len _normal _point) (message `/Game/Blueprints/edge/edgeInterface.intersection` _array_element self))
    (if (and (< _len (`local.len min`)) (< 0.0 _len))
      (set `local.len min` _len)
      (set `local.normal min` _normal)
      (set `local.point min` _point)
      (set `local.edge min` _array_index)))
  ;[1 1 1] если пересечений нет
  (if (< (`local.edge min`) _returnvalue)
    ;[1 1 1] если есть
    (set `self.len` (`local.len min`))
    (bind (_pointout _vectorout) (message `/Game/Blueprints/shader/ShaderInterface.shader` (`|GetArrayItem` edges) (`local.point min`) (`self.vector`) (`local.normal min`)))
    (bind _returnvalue_2 (`|GenericCreateObject` "ray_C" self 1.0 _pointout _vectorout))
    (return _returnvalue_2)
    (else
      (set `self.len` -1.0)
      (return self))))